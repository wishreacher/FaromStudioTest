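; BP_Rifle is an assault rifle pickup that becomes the player character's current ranged weapon.
; Overlapping its Box shows a W_PickUp prompt widget, and leaving removes it.
; The PickUp event clears the prompt, sets the player as owner, stores itself in CurrentRangeWeapon and snaps onto the mesh's WeaponSocket.
; If a weapon is already held, it first calls detach and moves to the player's location.
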(event `/Game/Weapons/AssaultRifle/BPI_RangeWeapon.Pick Up`
  (bind _pickup_widget (`self.PickUp Widget`))
  (bind _asfarom_studio_test_character (cast `FaromStudioTestCharacter` (`GameplayStatics.GetPlayerCharacter` 0) :!pure true))
  (`/Engine/EditorBlueprintResources/StandardMacros.IsValid` _pickup_widget
    (:`Is Valid`
      (`Widget.RemoveFromParent` _pickup_widget))
    (:`Is Not Valid`
      _))
  (`self.SetOwner` _asfarom_studio_test_character)
  (`/Engine/EditorBlueprintResources/StandardMacros.IsValid` (`FaromStudioTestCharacter.CurrentRangeWeapon` _asfarom_studio_test_character)
    (:`Is Valid`
      (`self.K2_DetachFromActor` "KeepRelative")
      (`self.K2_SetActorLocation` (`self.K2_GetActorLocation` _asfarom_studio_test_character)))
    (:`Is Not Valid`
      _))
  (set `FaromStudioTestCharacter.CurrentRangeWeapon` self _asfarom_studio_test_character)
  (`self.K2_AttachToComponent` (`Character.Mesh` (cast `FaromStudioTestCharacter` (`GameplayStatics.GetPlayerCharacter` 0) :!pure true)) "WeaponSocket" "SnapToTarget" "SnapToTarget" "SnapToTarget"))

(event `self.Box.OnComponentBeginOverlap`
  (params (OverlappedComponent :type "PrimitiveComponent Object Reference") (OtherActor :type "Actor Object Reference") (OtherComp :type "PrimitiveComponent Object Reference") (OtherBodyIndex :type Integer) (bFromSweep :type Boolean) (SweepResult :type "HitResult Structure (by ref)"))
  (bind _returnvalue (`|CreateWidget` "/Game/UI/W_PickUp.W_PickUp_C"))
  (set `self.PickUp Widget` _returnvalue)
  (`UserWidget.AddToViewport` _returnvalue 0))

(event `self.Box.OnComponentEndOverlap`
  (params (OverlappedComponent :type "PrimitiveComponent Object Reference") (OtherActor :type "Actor Object Reference") (OtherComp :type "PrimitiveComponent Object Reference") (OtherBodyIndex :type Integer))
  (bind _pickup_widget (`self.PickUp Widget`))
  (`/Engine/EditorBlueprintResources/StandardMacros.IsValid` _pickup_widget
    (:`Is Valid`
      (`Widget.RemoveFromParent` _pickup_widget))))

(fn `UserConstructionScript`)